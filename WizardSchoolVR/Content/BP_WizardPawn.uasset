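; BP_WizardPawn is a wizard pawn that tracks interactable items near its left and right hand controllers.
; Each hand has an interaction bubble whose begin and end overlap events filter for InteractableItem actors.
; Both events call UpdateClosestInteractableToHand with that bubble and a left-controller flag, so the closest-item selection refreshes only when overlaps change.
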(event OnComponentBeginOverlap(R_InteractionBubble)
  (params (OverlappedComponent :type Primitive%20Component%20Object%20Reference) (OtherActor :type Actor%20Object%20Reference) (OtherComp :type Primitive%20Component%20Object%20Reference) (OtherBodyIndex :type Integer) (bFromSweep :type Boolean) (SweepResult :type Hit%20Result%20Structure%20%28by%20ref%29))
  (Utilities|Casting|CastToInteractableItem OtherActor)
  (Class|WizardPawn|UpdateClosestInteractabletoHand (Variables|Default|GetR_InteractionBubble) false))

(event OnComponentBeginOverlap(L_InteractionBubble)
  (params (OverlappedComponent :type Primitive%20Component%20Object%20Reference) (OtherActor :type Actor%20Object%20Reference) (OtherComp :type Primitive%20Component%20Object%20Reference) (OtherBodyIndex :type Integer) (bFromSweep :type Boolean) (SweepResult :type Hit%20Result%20Structure%20%28by%20ref%29))
  (Utilities|Casting|CastToInteractableItem OtherActor)
  (Class|WizardPawn|UpdateClosestInteractabletoHand (Variables|Default|GetL_InteractionBubble) true))

(event OnComponentEndOverlap(L_InteractionBubble)
  (params (OverlappedComponent :type Primitive%20Component%20Object%20Reference) (OtherActor :type Actor%20Object%20Reference) (OtherComp :type Primitive%20Component%20Object%20Reference) (OtherBodyIndex :type Integer))
  (Utilities|Casting|CastToInteractableItem OtherActor)
  (Class|WizardPawn|UpdateClosestInteractabletoHand (Variables|Default|GetL_InteractionBubble) true))

(event OnComponentEndOverlap(R_InteractionBubble)
  (params (OverlappedComponent :type Primitive%20Component%20Object%20Reference) (OtherActor :type Actor%20Object%20Reference) (OtherComp :type Primitive%20Component%20Object%20Reference) (OtherBodyIndex :type Integer))
  (Utilities|Casting|CastToInteractableItem OtherActor)
  (Class|WizardPawn|UpdateClosestInteractabletoHand (Variables|Default|GetR_InteractionBubble) false))

(event EventBeginPlay)

(event Collision|EventActorBeginOverlap
  (params (OtherActor :type Actor%20Object%20Reference)))

(fn ConstructionScript)